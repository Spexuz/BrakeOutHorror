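; BP_Paul is the first-person player character, with Enhanced Input movement, look, FOV zoom with audio, and a toggled flashlight.
; It adds its mapping context on controller change and drives zoom through a timeline.
; Tick starts a walk or idle camera shake from velocity and CanJump to fake headbob.
; Movement plays and stops a footsteps timeline, but the sphere-trace dirt footstep sound hangs off an unreached Footsteps_TL node.
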(event `self.ReceiveControllerChanged`
  (params (OldController :type "Controller Object Reference") (NewController :type "Controller Object Reference"))
  ;[1 1 1 0.5] Map IMC to Character
  (bind _asplayer_controller (cast `PlayerController` NewController))
  (message `EnhancedInputSubsystemInterface.AddMappingContext` (pcsubsystem `EnhancedInputLocalPlayerSubsystem` _asplayer_controller) "/Game/Assets/Player/PLAYER_Controller/Inputs/IMC_Paul.IMC_Paul" 0 (struct)))

(event `EnhancedInput|/Game/Assets/Player/PLAYER_Controller/Inputs/IA_Move`
  (params (ActionValue :type "Vector2D Structure") (ElapsedSeconds :type "Float (double-precision)") (TriggeredSeconds :type "Float (double-precision)") (InputAction :type "InputAction Object Reference" :default "/Game/Assets/Player/PLAYER_Controller/Inputs/IA_Move.IA_Move"))
  (bind (_returnvalue_roll _returnvalue_pitch _returnvalue_yaw) (`KismetMathLibrary.BreakRotator` (`self.GetControlRotation`)))
  ;[1 1 1 0.5] Movement Center
  ;; WASD
  (:`Triggered`
    (`self.AddMovementInput` (`KismetMathLibrary.GetRightVector` (`KismetMathLibrary.MakeRotator` _returnvalue_roll 0.0 _returnvalue_yaw)) ActionValue_X)
    ;;; Footstep Check
    (if (> (`KismetMathLibrary.VSize` (`self.GetVelocity`)) 0.0) :!label _label
      (`TimelineComponent.Play` (`self.Footsteps_TL`))))
  (:`Completed`
    (`TimelineComponent.Stop` (`self.Footsteps_TL`) :!label _label_2)))

(event `EnhancedInput|/Game/Assets/Player/PLAYER_Controller/Inputs/IA_Zoom`
  (params (ActionValue :type Boolean) (ElapsedSeconds :type "Float (double-precision)") (TriggeredSeconds :type "Float (double-precision)") (InputAction :type "InputAction Object Reference" :default "/Game/Assets/Player/PLAYER_Controller/Inputs/IA_Zoom.IA_Zoom"))
  ;[1 1 1 0.5] Action Center
  ;; Camera Zoom - FOV
  (:`Started`
    (if (`AudioComponent.IsPlaying` (`self.ZoomAudio`))
      (bind (_direction _zoom_curve) (`Timeline|Timeline` :!label _label_3)
        (:`Update`
          (`CameraComponent.SetFieldOfView` (`self.FirstPersonCamera`) (`KismetMathLibrary.Lerp` 90.0 45.0 _zoom_curve))))
      (else
        (`AudioComponent.Play` (`self.ZoomAudio`) 0.0)
        (goto _label_3))))
  (:`Completed`
    (if (`AudioComponent.IsPlaying` (`self.ZoomAudio`))
      (goto _label_3 :!via `Reverse`)
      (else
        (`AudioComponent.Play` (`self.ZoomAudio`) 0.0)
        (goto _label_3 :!via `Reverse`)))))

(event `EnhancedInput|/Game/Assets/Player/PLAYER_Controller/Inputs/IA_Move`
  (params (ActionValue :type "Vector2D Structure") (ElapsedSeconds :type "Float (double-precision)") (TriggeredSeconds :type "Float (double-precision)") (InputAction :type "InputAction Object Reference" :default "/Game/Assets/Player/PLAYER_Controller/Inputs/IA_Move.IA_Move"))
  (bind (_returnvalue_roll _returnvalue_pitch _returnvalue_yaw) (`KismetMathLibrary.BreakRotator` (`self.GetControlRotation`)))
  ;[1 1 1 0.5] Movement Center
  ;; WASD
  (:`Triggered`
    (`self.AddMovementInput` (`KismetMathLibrary.GetForwardVector` (`KismetMathLibrary.MakeRotator` 0.0 0.0 _returnvalue_yaw)) ActionValue_Y)
    (goto _label))
  (:`Completed`
    (goto _label_2)))

(event `EnhancedInput|/Game/Assets/Player/PLAYER_Controller/Inputs/IA_LookXY`
  (params (ActionValue :type "Vector2D Structure") (ElapsedSeconds :type "Float (double-precision)") (TriggeredSeconds :type "Float (double-precision)") (InputAction :type "InputAction Object Reference" :default "/Game/Assets/Player/PLAYER_Controller/Inputs/IA_LookXY.IA_LookXY"))
  ;[1 1 1 0.5] Movement Center
  ;; WASD
  ;;; Camera XY
  (:`Triggered`
    (`self.AddControllerYawInput` ActionValue_X)
    (`self.AddControllerPitchInput` ActionValue_Y)))

(event `EnhancedInput|/Game/Assets/Player/PLAYER_Controller/Inputs/IA_Flashlight`
  (params (ActionValue :type Boolean) (ElapsedSeconds :type "Float (double-precision)") (TriggeredSeconds :type "Float (double-precision)") (InputAction :type "InputAction Object Reference" :default "/Game/Assets/Player/PLAYER_Controller/Inputs/IA_Flashlight.IA_Flashlight"))
  (bind _spotlight (`self.SpotLight`))
  (bind _returnvalue (`SceneComponent.K2_GetComponentLocation` (`self.SpotLight`)))
  ;[1 1 1 0.5] Action Center
  (:`Started`
    (`/Engine/EditorBlueprintResources/StandardMacros.FlipFlop`
      (:`A`
        (`GameplayStatics.PlaySoundAtLocation` "/Game/Assets/SoundFX/Interactable_Sounds/flashlight-clicking-on-105809__1_.flashlight-clicking-on-105809__1_" _returnvalue (struct) 1.0 1.0 0.0 null null null null)
        (`KismetSystemLibrary.Delay` 0.2)
        (`SceneComponent.SetVisibility` _spotlight true false))
      (:`B`
        (`GameplayStatics.PlaySoundAtLocation` "/Game/Assets/SoundFX/Interactable_Sounds/flashlight-clicking-on-105809__1_.flashlight-clicking-on-105809__1_" _returnvalue (struct) 1.0 1.0 0.0 null null null null)
        (`KismetSystemLibrary.Delay` 0.2)
        (`SceneComponent.SetVisibility` _spotlight false false)))))

(event `self.ReceiveTick`
  (params (DeltaSeconds :type "Float (single-precision)"))
  ;[1 1 1 0.5] Headbobbing
  ;; Call Event
  (`self.Headbob`))

(event `Headbob`
  (bind _returnvalue (`GameplayStatics.GetPlayerController` 0))
  ;[1 1 1 0.5] Headbobbing
  (if (and (> (`KismetMathLibrary.VSize` (`self.GetVelocity`)) 0.0) (`self.CanJump`))
    (`PlayerController.ClientStartCameraShake` :`self` _returnvalue :`Shake` "/Game/Assets/Player/PLAYER_Controller/Headbob/CS_Walk.CS_Walk_C")
    (else
      (`PlayerController.ClientStartCameraShake` :`self` _returnvalue :`Shake` "/Game/Assets/Player/PLAYER_Controller/Headbob/CS_Idle.CS_Idle_C"))))

(fn `TraceFootsteps`
  (returns (Finished :type Boolean))
  (bind _returnvalue (`self.K2_GetActorLocation`))
  (bind _capsulecomponent (`self.CapsuleComponent`))
  (bind (_outhit _returnvalue_2) (`KismetSystemLibrary.SphereTraceSingle` _returnvalue (`KismetMathLibrary.MakeVector` (.x _returnvalue) (.y _returnvalue) (- (.z _returnvalue) (`CapsuleComponent.GetScaledCapsuleHalfHeight` _capsulecomponent))) (`CapsuleComponent.GetScaledCapsuleRadius` _capsulecomponent) "TraceTypeQuery1"))
  (return _returnvalue_2))

(fn `TryFootsteps`
  (bind _finished (`self.TraceFootsteps`))
  (if _finished
    (`GameplayStatics.PlaySoundAtLocation` "/Game/Assets/SoundFX/Footsteps_Sounds/Dirt/DirtFootStep.DirtFootStep" (`self.K2_GetActorLocation`) (struct) 1.0 1.0 0.0 null null null null)))

(fn `UserConstructionScript`)