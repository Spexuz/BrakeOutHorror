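; BP_A_Door_Locked is an interactable house door that stays locked and reveals this when tried.
; Its first interaction switches the Status enum to ShowLock, plays a rattle sound and runs the DoorMechanics timeline, whose DoorShaking track drives the Cube's yaw.
; Later interactions only reverse that timeline, without sound.
; ShowInfo sets the HUD prompt from Status, changing "Open Door" to "Door is Locked".
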(event `self.InteractInterface`
  (switch `/Game/Assets/Game_Assets/House/Doors/EN_DoorLocked` (`self.Status`)
    (:`NewEnumerator0`
      (set `self.Status` "NewEnumerator1")
      (`GameplayStatics.PlaySound2D` "/Game/Assets/SoundFX/Door_Sounds/Door_Rattle.Door_Rattle" 1.0 1.0 0.0 null null)
      (bind (_direction _doorshaking) (`Timeline|Door Mechanics` :!label _label)
        (:`Update`
          (`SceneComponent.K2_SetRelativeRotation` (`self.Cube`) (`KismetMathLibrary.MakeRotator` 0.0 0.0 _doorshaking) false false))))
    (:`NewEnumerator1`
      (set `self.Status` "NewEnumerator1")
      (goto _label :!via `Reverse`))))

(event `self.ShowInfo`
  (params (HUD :type "/Game/Assets/UI/UI/WB_Interact_Interface Object Reference"))
  (switch `/Game/Assets/Game_Assets/House/Doors/EN_DoorLocked` (`self.Status`)
    (:`NewEnumerator0`
      (`/Game/Assets/UI/UI/WB_Interact_Interface.SetInfoText` HUD "Open Door"))
    (:`NewEnumerator1`
      (`/Game/Assets/UI/UI/WB_Interact_Interface.SetInfoText` HUD "Door is Locked"))))

(fn `UserConstructionScript`)