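; BP_A_Door is a house door that the player opens and closes through an interaction interface.
; InteractInterface flips the Open/Closed Status, plays the matching 2D sound, and plays or reverses the DoorMechanics timeline, which drives the Cube's relative yaw.
; ShowInfo sets the HUD prompt to open or close the door according to the current Status.
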(event `/Game/Assets/Player/PLAYER_Controller/Inputs/I_Interactable.InteractInterface`
  (switch `/Game/Assets/Game_Assets/House/Doors/EN_Door` (`self.Status`)
    (:`NewEnumerator0`
      (set `self.Status` "NewEnumerator1")
      (`GameplayStatics.PlaySound2D` "/Game/Assets/SoundFX/Door_Sounds/Door_Open.Door_Open" 1.0 1.0 0.0 null null)
      (bind (_direction _door_z_rotation) (`Timeline|Door Mechanics` :!label _label)
        (:`Update`
          (`SceneComponent.K2_SetRelativeRotation` (`self.Cube`) (`KismetMathLibrary.MakeRotator` 0.0 0.0 _door_z_rotation) false false))))
    (:`NewEnumerator1`
      (set `self.Status` "NewEnumerator0")
      (`GameplayStatics.PlaySound2D` "/Game/Assets/SoundFX/Door_Sounds/Door_Close.Door_Close" 1.0 1.0 0.0 null null)
      (goto _label :!via `Reverse`))))

(event `/Game/Assets/Player/PLAYER_Controller/Inputs/I_Interactable.ShowInfo`
  (params (HUD :type "/Game/Assets/UI/UI/WB_Interact_Interface Object Reference"))
  (switch `/Game/Assets/Game_Assets/House/Doors/EN_Door` (`self.Status`)
    (:`NewEnumerator0`
      (`/Game/Assets/UI/UI/WB_Interact_Interface.SetInfoText` HUD "Press \"F\" To Open Door"))
    (:`NewEnumerator1`
      (`/Game/Assets/UI/UI/WB_Interact_Interface.SetInfoText` HUD "Press \"F\" To Close Door"))))

(fn `UserConstructionScript`)